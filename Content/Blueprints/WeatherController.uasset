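; Weather controller that runs a timed clouds-and-rain sequence on BeginPlay.
; Delays raise the target cloud opacity, toggle rain on and off, then lower the target.
; Each Tick checks sky opacity and the MP_Global RainLevel against their targets, then refreshes the sky material.
; Outside tolerance, opacity jumps to target plus ChangeRate and RainLevel is set to ChangeRate itself, so neither steps gradually.
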(event `self.ReceiveBeginPlay`
  (`KismetSystemLibrary.Delay` 0.2)
  (`KismetSystemLibrary.Delay` 5.0)
  (set `self.TargetCloudOpacity` 3.0)
  (`KismetSystemLibrary.Delay` 10.0)
  (`self.ToggleRain` true)
  (`KismetSystemLibrary.Delay` 30.0)
  (`self.ToggleRain` false)
  (set `self.TargetCloudOpacity` 0.7))

(event `self.ReceiveTick`
  (params (DeltaSeconds :type "Float (single-precision)"))
  (bind _targetcloudopacity (`self.TargetCloudOpacity`))
  (bind _returnvalue (> (`KismetMathLibrary.Abs` (- (`/Engine/EngineSky/BP_Sky_Sphere.Cloud opacity` (`self.Sky`)) _targetcloudopacity)) 0.1))
  (if _returnvalue
    (set `/Engine/EngineSky/BP_Sky_Sphere.Cloud opacity` (+ _targetcloudopacity (* (`self.ChangeRate`) (`KismetMathLibrary.SelectFloat` 1.0 -1.0 _returnvalue)) 0.0) (`self.Sky`)))
  (bind _returnvalue_2 (`KismetMaterialLibrary.GetScalarParameterValue` "/Game/Blueprints/MP_Global.MP_Global" "RainLevel"))
  (bind _returnvalue_3 (> (`KismetMathLibrary.Abs` (- (`self.TargetRainLevel`) _returnvalue_2)) 0.1))
  (if _returnvalue_3
    (`KismetMaterialLibrary.SetScalarParameterValue` "/Game/Blueprints/MP_Global.MP_Global" "RainLevel" (* (`self.ChangeRate`) (`KismetMathLibrary.SelectFloat` 1.0 -1.0 _returnvalue_3))))
  (`/Engine/EngineSky/BP_Sky_Sphere.RefreshMaterial` (`self.Sky`)))

(fn `UserConstructionScript`)